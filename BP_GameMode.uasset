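; Game mode that runs a grid-based Snake game with score and end-screen widgets.
; Setup spawns a ground grid, the first tail box and a randomly placed food actor.
; A looping timer moves the snake by shifting a position array onto box actors, speeding up with length within limits.
; Eating food grows the snake, relocates food and updates score; leaving bounds or self-collision pauses the game and shows the end screen.
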(event `self.ReceiveBeginPlay`
  (`WidgetBlueprintLibrary.SetInputMode_GameOnly` (`GameplayStatics.GetPlayerController` 0))
  (bind _returnvalue (`|CreateWidget` "/Game/BWI_Score.BWI_Score_C"))
  (bind _output_get (set `self.Score UI` _returnvalue))
  (`UserWidget.AddToViewport` _output_get 0)
  (`self.Setup`)
  (`self.UpdateTimer`))

(fn `CanGoToPosition?`
  (params (Position :type "Vector Structure"))
  (returns (CanGoBool :type Boolean))
  (locals (CanGo :type Boolean :default true) (NewPosition :type "Vector Structure"))
  (bind _output_get (set `local.NewPosition` Position))
  (if (or (or (>= (.x _output_get) (`self.Width`)) (< (.x _output_get) 0.0)) (or (>= (.y _output_get) (`self.Height`)) (< (.y _output_get) 0.0)))
    (return false)
    (else
      (for _array_element (`self.TailPosition`)
        (if (< (`KismetMathLibrary.VSize` (- _array_element (`local.NewPosition`))) 1.0)
          (set `local.CanGo` false)))
      (return (`local.CanGo`)))))

(fn `Death`
  (bind _returnvalue (`GameplayStatics.GetPlayerController` 0))
  (`GameplayStatics.SetGamePaused` true)
  (bind _returnvalue_2 (`|CreateWidget` "/Game/BWI_End.BWI_End_C"))
  (`UserWidget.AddToViewport` _returnvalue_2 0)
  (`WidgetBlueprintLibrary.SetInputMode_UIOnlyEx` _returnvalue _returnvalue_2 "DoNotLock" true)
  (set `PlayerController.bShowMouseCursor` true _returnvalue))

(fn `GetRandomFoodPosition`
  (returns (FoodPositionOutput :type "Vector Structure"))
  (bind _output_get (set `self.Food Position` (`KismetMathLibrary.MakeVector` (`KismetMathLibrary.Conv_IntToDouble` (`KismetMathLibrary.RandomIntegerInRange` (`self.MinDistanceFromTheEdges`) (- (- (`self.Width`) 1) (`self.MinDistanceFromTheEdges`)))) (`KismetMathLibrary.Conv_IntToDouble` (`KismetMathLibrary.RandomIntegerInRange` (`self.MinDistanceFromTheEdges`) (- (- (`self.Height`) 1) (`self.MinDistanceFromTheEdges`)))))))
  (return _output_get))

(fn `Grow`
  (params (Position :type "Vector Structure"))
  (`KismetArrayLibrary.Array_Insert` (`self.TailPosition`) Position)
  (bind _returnvalue (`|SpawnActorFromClass` "/Game/BP_TailBox.BP_TailBox_C" (`KismetMathLibrary.MakeTransform` (* Position (`self.Scale`))) "Undefined" "MultiplyWithRoot" null null))
  (`KismetArrayLibrary.Array_Add` (`self.TailBoxes`) _returnvalue))

(fn `Setup`
  (`|ExecutionSequence`
    (:`then_0`
      (for _index (range (`self.Height`))
        (set `self.Y` _index)
        (for _index_2 (range (`self.Width`))
          (set `self.X` _index_2)
          (`|SpawnActorFromClass` "/Game/BP_GroundBox.BP_GroundBox_C" (`KismetMathLibrary.MakeTransform` (`KismetMathLibrary.MakeVector` (`KismetMathLibrary.Conv_IntToDouble` (* (`self.X`) (`self.Scale`))) (`KismetMathLibrary.Conv_IntToDouble` (* (`self.Y`) (`self.Scale`))) (`KismetMathLibrary.Conv_IntToDouble` (* (`self.Scale`) -1)))) "Undefined" "MultiplyWithRoot" null null))))
    (:`then_1`
      (bind _output_get (set `self.InitialPosition` (`KismetMathLibrary.MakeVector` (`KismetMathLibrary.Conv_IntToDouble` (/ (`self.Height`) 2)) (`KismetMathLibrary.Conv_IntToDouble` (/ (`self.Width`) 2)))))
      (`self.Grow` _output_get))
    (:`then_2`
      (bind _foodpositionoutput (`self.GetRandomFoodPosition`))
      (bind (_returnvalue_x _returnvalue_y) (`KismetMathLibrary.BreakVector` (* _foodpositionoutput (`self.Scale`))))
      (bind _returnvalue (`|SpawnActorFromClass` "/Game/BP_Food.BP_Food_C" (`KismetMathLibrary.MakeTransform` (`KismetMathLibrary.MakeVector` _returnvalue_x _returnvalue_y (`KismetMathLibrary.Conv_IntToDouble` (`self.Scale`)))) "Undefined" "MultiplyWithRoot" null null))
      (set `self.FoodBox` _returnvalue))))

(fn `UpdateTail`
  (locals (NewFirstBoxPosition :type "Vector Structure"))
  (bind _tailposition (`self.TailPosition`))
  (bind _output_get (set `local.NewFirstBoxPosition` (+ (`self.Direction`) (`|GetArrayItem` (`self.TailPosition`)))))
  (bind _cangobool (`self.CanGoToPosition?` _output_get))
  (if _cangobool
    (if (< (`KismetMathLibrary.VSize` (- (`local.NewFirstBoxPosition`) (`self.Food Position`))) 1.0)
      (`self.Grow` (`local.NewFirstBoxPosition`))
      (bind _foodpositionoutput (`self.GetRandomFoodPosition`))
      (bind (_returnvalue_x _returnvalue_y) (`KismetMathLibrary.BreakVector` (* _foodpositionoutput (`self.Scale`))))
      (`self.K2_SetActorLocation` (`self.FoodBox`) (`KismetMathLibrary.MakeVector` _returnvalue_x _returnvalue_y (`KismetMathLibrary.Conv_IntToDouble` (`self.Scale`))) false false)
      (bind _result (`/Engine/EditorBlueprintResources/StandardMacros.IncrementInt` (`self.Score`))
        (:`  `
          (`/Game/BWI_Score.UpdateScore` (`self.Score UI`) _result)
          (`self.UpdateTimer`)))
      (else
        (`KismetArrayLibrary.Array_Remove` _tailposition (`KismetArrayLibrary.Array_LastIndex` _tailposition))
        (`KismetArrayLibrary.Array_Insert` (`self.TailPosition`) (`local.NewFirstBoxPosition`))
        (for (_array_element _array_index) (`self.TailBoxes`)
          (`self.K2_SetActorLocation` _array_element (* (`|GetArrayItem` (`self.TailPosition`) _array_index) (`self.Scale`)) false false))))
    (else
      (`self.Death`))))

(fn `UpdateTimer`
  (bind _returnvalue (`KismetMathLibrary.FMax` (* (`KismetMathLibrary.FMin` (/ (`KismetArrayLibrary.Array_Length` (`self.TailBoxes`)) (`self.LengthMaxTimerSpeed`)) 1.0) (`self.MaxTimerSpeed`)) (`self.MinTimerSpeed`)))
  (`KismetSystemLibrary.PrintString` (`KismetStringLibrary.Conv_DoubleToString` _returnvalue))
  (`KismetSystemLibrary.K2_ClearAndInvalidateTimerHandle` (`self.Timer`))
  (bind _returnvalue_2 (`KismetSystemLibrary.K2_SetTimer` null "UpdateTail" (/ 1.0 _returnvalue) true))
  (set `self.Timer` _returnvalue_2))

(fn `UserConstructionScript`)