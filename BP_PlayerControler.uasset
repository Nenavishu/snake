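; Player controller that turns four-way key input into movement direction changes for a tailed, snake-style game.
; BeginPlay adds the game's Enhanced Input mapping context, and each up, down, left or right action passes an axis vector to SetDirecion.
; That function rejects repeats and reversals using vector-length checks on the sum and difference with the current direction.
; Accepted turns are written to BP_GameMode, which then updates its tail and timer.
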(event `self.ReceiveBeginPlay`
  (`EnhancedInputSubsystemInterface.AddMappingContext` (subsystem `EnhancedInputLocalPlayerSubsystem`) "/Game/Input/IMC_GAME.IMC_GAME" 0 (struct)))

(event `EnhancedInput|/Game/Input/IA_UP`
  (params (ActionValue :type Boolean) (ElapsedSeconds :type "Float (double-precision)") (TriggeredSeconds :type "Float (double-precision)") (InputAction :type "InputAction Object Reference" :default "/Game/Input/IA_UP.IA_UP"))
  (:`Started`
    (`self.SetDirecion` (`KismetMathLibrary.MakeVector` 1.0))))

(event `EnhancedInput|/Game/Input/IA_DOWN`
  (params (ActionValue :type Boolean) (ElapsedSeconds :type "Float (double-precision)") (TriggeredSeconds :type "Float (double-precision)") (InputAction :type "InputAction Object Reference" :default "/Game/Input/IA_DOWN.IA_DOWN"))
  (:`Started`
    (`self.SetDirecion` (`KismetMathLibrary.MakeVector` -1.0))))

(event `EnhancedInput|/Game/Input/IA_RIGHT`
  (params (ActionValue :type Boolean) (ElapsedSeconds :type "Float (double-precision)") (TriggeredSeconds :type "Float (double-precision)") (InputAction :type "InputAction Object Reference" :default "/Game/Input/IA_RIGHT.IA_RIGHT"))
  (:`Started`
    (`self.SetDirecion` (`KismetMathLibrary.MakeVector` 0.0 1.0))))

(event `EnhancedInput|/Game/Input/IA_LEFT`
  (params (ActionValue :type Boolean) (ElapsedSeconds :type "Float (double-precision)") (TriggeredSeconds :type "Float (double-precision)") (InputAction :type "InputAction Object Reference" :default "/Game/Input/IA_LEFT.IA_LEFT"))
  (:`Started`
    (`self.SetDirecion` (`KismetMathLibrary.MakeVector` 0.0 -1.0))))

(fn `SetDirecion`
  (params (`New Direction` :type "Vector Structure"))
  (bind _asbp_game_mode (cast `/Game/BP_GameMode` (`GameplayStatics.GetGameMode`)))
  (bind _direction (`/Game/BP_GameMode.Direction` _asbp_game_mode))
  (if (and (>= (`KismetMathLibrary.VSize` (+ _direction `New Direction`)) 1.0) (>= (`KismetMathLibrary.VSize` (- _direction `New Direction`)) 1.0))
    (set `/Game/BP_GameMode.Direction` `New Direction` _asbp_game_mode)
    (`/Game/BP_GameMode.UpdateTail` _asbp_game_mode)
    (`/Game/BP_GameMode.UpdateTimer` _asbp_game_mode)))

(fn `UserConstructionScript`)